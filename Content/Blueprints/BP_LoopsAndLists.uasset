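; Demo actor Blueprint showing loop techniques, started on BeginPlay, using on-screen text and BP_Tree actors.
; A while loop prints a color-cycled countdown with timestamps, all at once.
; An endless Delay-based loop repeatedly triggers LoopArrayOverTime, which randomizes tree yaw one by one via a delayed index loop.
; ChangeTrees rotates every tree at once with a for-each but is never called here.
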(event Custom|SimpleLoop
  (Development|PrintText "Inside Simple Loop, waiting 3 seconds" :!label _label)
  (CallFunction|LoopArrayOverTime)
  (Utilities|FlowControl|Delay 3.0)
  (goto _label))

(event Custom|WhileLoop%20Function
  (bind _colors (Variables|Default|GetColors))
  ;[0.15 0.15 0.15 0.5] While Loop
  (while (> (Variables|Default|GetWhileCounter) 0)
    (Development|PrintText (Utilities|Text|FormatText "This is loop {count}. Ran after {seconds} seconds." (Variables|Default|GetWhileCounter) (Utilities|Text|ToText(Float) (Utilities|Time|GetRealTimeSeconds) "HalfToEven" false true 1 324 3)) true true (Utilities|Array|Get(acopy) _colors (Math|Integer|%(Integer) (Variables|Default|GetWhileCounter) (Utilities|Array|Length _colors))) 2e+01)
    (Math|Integer|DecrementInt (Variables|Default|GetWhileCounter))))

(event Custom|Change%20Trees
  (bind _outactors (Actor|GetAllActorsOfClass "/Game/Blueprints/BP_Tree.BP_Tree_C"))
  (for _array_element _outactors
    (Transformation|SetActorRelativeRotation _array_element (Math|Rotator|MakeRotator 0.0 0.0 (Math|Random|RandomFloatinRange 0.0 3.6e+02)))))

(event Custom|LoopArrayOverTime
  (bind _outactors (Actor|GetAllActorsOfClass "/Game/Blueprints/BP_Tree.BP_Tree_C"))
  (if (< (Variables|Default|GetOverTImeIndex) (Utilities|Array|Length _outactors)) :!label _label
    (Transformation|SetActorRotation (Utilities|Array|Get(acopy) _outactors (Variables|Default|GetOverTImeIndex)) (Math|Rotator|MakeRotator 0.0 0.0 (Math|Random|RandomFloatinRange 0.0 3.6e+02)))
    (Math|Integer|IncrementInt (Variables|Default|GetOverTImeIndex)
      (:%20%20
        (Utilities|FlowControl|Delay 0.2)
        (goto _label)))
    (else
      (Variables|Default|SetOverTImeIndex 0))))

(event EventBeginPlay
  (CallFunction|WhileLoopFunction)
  (CallFunction|SimpleLoop))

(fn ConstructionScript)