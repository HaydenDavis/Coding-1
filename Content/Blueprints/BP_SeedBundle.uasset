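; BP_SeedBundle is a pickup that gives the third-person character a random number of seeds on overlap and plays a sound.
; The seed amount is rolled on BeginPlay.
; When RespawnSeeds is set, a collected bundle rerolls its amount and hides for a random delay before reappearing, with a Hidden flag blocking pickup meanwhile; otherwise it destroys itself.
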(event Custom|RespawnSeed
  (Rendering|SetActorHiddenInGame true)
  (Variables|Default|SetHidden? true)
  (Utilities|FlowControl|Delay (Math|Random|RandomFloatinRange 5.0 15.0))
  (Rendering|SetActorHiddenInGame false)
  (Variables|Default|SetHidden? false))

(event Custom|RandomizeSeedAmount
  (Variables|Default|SetSeedAmount (Math|Random|RandomIntegerinRange 1 10)))

(event EventBeginPlay
  (CallFunction|RandomizeSeedAmount))

(event Collision|EventActorBeginOverlap
  (params (OtherActor :type Actor%20Object%20Reference))
  (if (not (Variables|Default|GetHidden?))
    (bind _asbp_third_person_character (Utilities|Casting|CastToBP_ThirdPersonCharacter OtherActor))
    (Default|CollectSeeds _asbp_third_person_character (Variables|Default|GetSeedAmount))
    (Audio|PlaySoundatLocation "/Engine/VREditor/Sounds/UI/Foliage_Placed.Foliage_Placed" (Transformation|GetActorLocation) "0, 0, 0" 1.0 1.0 0.0 0 0 0 0)
    (if (Variables|Default|GetRespawnSeeds?)
      (CallFunction|RandomizeSeedAmount)
      (CallFunction|RespawnSeed)
      (else
        (Actor|DestroyActor)))))

(fn ConstructionScript)