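; BP_Flower is a flower that picks a random mesh on spawn and grows over time.
; BeginPlay sets SMFlower to one of five flower meshes, including daisy, dandelion, hyacinth and rose, then starts TheGrowLoop.
; The loop uses a DoN node with a random count to repeat delayed Grow calls at random intervals.
; Each Grow adds a random increment to the mesh's relative scale.
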(event Custom|Grow
  (bind _sm_flower (Variables|Default|GetSM_Flower))
  (Transformation|SetRelativeScale3D _sm_flower (+ (Variables|/Script/Engine.SceneComponent|GetRelativeScale3D _sm_flower) (Math|Random|RandomFloatinRange 0.1 0.3))))

(event Custom|The%20Grow%20Loop
  (bind _output_get (Variables|Default|SetLoopCount (Math|Random|RandomIntegerinRange 1 3)))
  (bind _counter (Utilities|FlowControl|DoN _output_get :!label _label)
    (:Exit
      (Utilities|FlowControl|Delay (Math|Random|RandomFloatinRange 3.0 5.0))
      (CallFunction|Grow)
      (if (not (== (Variables|Default|GetLoopCount) _counter))
        (goto _label)))))

(event EventBeginPlay
  (bind _output_get (Variables|Default|SetFlowerTypes (Utilities|Array|MakeArray "/Game/DEMOFlowerpack/StaticMesh/SM_Daisy_Single.SM_Daisy_Single" "/Game/DEMOFlowerpack/StaticMesh/SM_Dandelion_Small.SM_Dandelion_Small" "/Game/DEMOFlowerpack/StaticMesh/SM_Hyacinth_PastellBlue_Big.SM_Hyacinth_PastellBlue_Big" "/Game/DEMOFlowerpack/StaticMesh/SM_Rose_Black_Open.SM_Rose_Black_Open" "/Game/DEMOFlowerpack/StaticMesh/SM_Rose_Red_Open.SM_Rose_Red_Open")))
  (Components|StaticMesh|SetStaticMesh (Variables|Default|GetSM_Flower) (.OutItem (Utilities|Array|Random _output_get)))
  (CallFunction|TheGrowLoop))

(fn ConstructionScript)