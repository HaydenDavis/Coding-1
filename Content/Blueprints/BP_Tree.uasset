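; BP_Tree is a tree actor that picks a random generic living or dead tree mesh at BeginPlay and grows in steps.
; A DoN-based loop runs a small random number of times, waiting a few seconds before each Grow call adds a random amount to the mesh's relative scale.
; After the final step it sets the mesh's collision to query and physics.
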(event Custom|Grow
  (bind _sm_tree (Variables|Default|GetSM_Tree))
  (Transformation|SetRelativeScale3D _sm_tree (+ (Variables|/Script/Engine.SceneComponent|GetRelativeScale3D _sm_tree) (Math|Random|RandomFloatinRange 0.2 0.4))))

(event Custom|The%20Grow%20Loop
  (bind _output_get (Variables|Default|SetLoopCount (Math|Random|RandomIntegerinRange 1 5)))
  (bind _counter (Utilities|FlowControl|DoN _output_get :!label _label)
    (:Exit
      (Utilities|FlowControl|Delay (Math|Random|RandomFloatinRange 3.0 5.0))
      (CallFunction|Grow)
      (if (== (Variables|Default|GetLoopCount) _counter)
        (Collision|SetCollisionEnabled (Variables|Default|GetSM_Tree) "QueryAndPhysics")
        (else
          (goto _label))))))

(event EventBeginPlay
  (bind _output_get (Variables|Default|SetTreeTypes (Utilities|Array|MakeArray "/Game/PolygonStarterPack/Meshes/SM_Generic_Tree_01.SM_Generic_Tree_01" "/Game/PolygonStarterPack/Meshes/SM_Generic_Tree_02.SM_Generic_Tree_02" "/Game/PolygonStarterPack/Meshes/SM_Generic_Tree_03.SM_Generic_Tree_03" "/Game/PolygonStarterPack/Meshes/SM_Generic_Tree_04.SM_Generic_Tree_04" "/Game/PolygonStarterPack/Meshes/SM_Generic_TreeDead_01.SM_Generic_TreeDead_01")))
  (Components|StaticMesh|SetStaticMesh (Variables|Default|GetSM_Tree) (.OutItem (Utilities|Array|Random _output_get)))
  (CallFunction|TheGrowLoop))

(fn ConstructionScript)