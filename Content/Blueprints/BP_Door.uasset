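; BP_Door is a key-gated door that swings open once when the player character enters its trigger box.
; The box overlap checks that BP_ThirdPersonCharacter holds at least one key, without consuming it, and otherwise prints a hint.
; A Timeline adds yaw to the mesh's relative rotation cached at BeginPlay, applies it as world rotation, and sets Opened to prevent replays.
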(event OnComponentBeginOverlap(Box)
  (params (OverlappedComponent :type Primitive%20Component%20Object%20Reference) (OtherActor :type Actor%20Object%20Reference) (OtherComp :type Primitive%20Component%20Object%20Reference) (OtherBodyIndex :type Integer) (bFromSweep :type Boolean) (SweepResult :type Hit%20Result%20Structure%20%28by%20ref%29))
  (bind _current_rotation (Variables|Default|GetCurrent%20Rotation))
  (bind _asbp_third_person_character (Utilities|Casting|CastToBP_ThirdPersonCharacter OtherActor))
  (if (> (Variables|/Game/ThirdPerson/Blueprints/BP_ThirdPersonCharacter.BP_ThirdPersonCharacter_C|GetTotal%20Keys _asbp_third_person_character) 0)
    (if (not (Variables|Default|GetOpened?))
      (bind _newtrack_0 (Timeline|Timeline PlayFromStart)
        (:Update
          (Transformation|SetWorldRotation (Variables|Default|GetSM_Bld_Door_01) (Math|Rotator|MakeRotator (.roll _current_rotation) (.pitch _current_rotation) (+ _newtrack_0 (.yaw _current_rotation))) false false)
          (Variables|Default|SetOpened? true))))
    (else
      (Development|PrintString "The player needs a key!"))))

(event EventBeginPlay
  (Variables|Default|SetCurrent%20Rotation (Variables|/Script/Engine.SceneComponent|GetRelativeRotation (Variables|Default|GetSM_Bld_Door_01))))

(event Collision|EventActorBeginOverlap
  (params (OtherActor :type Actor%20Object%20Reference)))

(event EventTick
  (params (DeltaSeconds :type Float%20%28single-precision%29)))

(fn ConstructionScript)