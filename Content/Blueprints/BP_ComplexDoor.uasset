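; Bunker door Blueprint that opens once four keys have been collected.
; Each KeyCollect call increments a counter, prints it and unhides the matching key mesh; the fourth triggers DoorOpen, which drives the door's Z position by timeline after a short delay.
; Overlapping the Cube component adds a congratulations dialogue widget on every overlap, without checking key count, and plays a second door timeline in reverse once via DoOnce.
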(event OnComponentBeginOverlap(Cube)
  (params (OverlappedComponent :type Primitive%20Component%20Object%20Reference) (OtherActor :type Actor%20Object%20Reference) (OtherComp :type Primitive%20Component%20Object%20Reference) (OtherBodyIndex :type Integer) (bFromSweep :type Boolean) (SweepResult :type Hit%20Result%20Structure%20%28by%20ref%29))
  (bind _door_location (Variables|Default|GetDoor%20location))
  (bind _returnvalue (UserInterface|CreateWidget "/Game/Widgets/W_Dialogue.W_Dialogue_C"))
  (bind _output_get (Variables|Default|SetWidget _returnvalue))
  (Rendering|Components|TextRender|SetText (Variables|/Game/Widgets/W_Dialogue.W_Dialogue_C|GetTextBlock_0 _output_get) "Congrats, you have found all four pieces to get into the bunker before the sun rises.")
  (UserInterface|Viewport|AddtoViewport (Variables|Default|GetWidget) 0)
  (Utilities|FlowControl|DoOnce false
    (:Completed
      (bind _newtrack_0 (Timeline|Timeline_0 ReverseFromEnd)
        (:Update
          (Transformation|SetRelativeLocation (Variables|Default|GetSM_Door) (Math|Vector|MakeVector (.x _door_location) (.y _door_location) (+ _newtrack_0 0.0)) false false))))))

(event Custom|Key%20Collect
  (Math|Integer|IncrementInt (Variables|Default|GetKeyCount)
    (:%20%20
      (Development|PrintText (Utilities|Text|FormatText "Total Keys in Door: {Total keys}" (Variables|Default|GetKeyCount)))
      (bind _index (Utilities|FlowControl|ForLoopwithBreak 1 4 :!label _label)
        (:LoopBody
          (if (== _index (Variables|Default|GetKeyCount))
            (goto _label Break)))
        (:Completed
          (Development|SetHiddeninGame (Utilities|Array|Get(acopy) (Utilities|Array|MakeArray (Variables|Default|GetSM_Key1) (Variables|Default|GetSM_Key2) (Variables|Default|GetSM_Key3) (Variables|Default|GetSM_Key4)) (- (Variables|Default|GetKeyCount) 1)) false false)
          (if (== (Variables|Default|GetKeyCount) 4)
            (CallFunction|DoorOpen)))))))

(event Custom|DoorOpen
  (bind _door_location (Variables|Default|GetDoor%20location))
  (Development|PrintText "Door is opening...")
  (Utilities|FlowControl|Delay 1.5)
  (bind _newtrack_0 (Timeline|Timeline PlayFromStart)
    (:Update
      (Transformation|SetRelativeLocation (Variables|Default|GetSM_Door) (Math|Vector|MakeVector (.x _door_location) (.y _door_location) (+ _newtrack_0 0.0)) false false))))

(event EventBeginPlay
  (Variables|Default|SetDoor%20location (.location (Transformation|GetRelativeTransform (Variables|Default|GetSM_Door)))))

(event Collision|EventActorBeginOverlap
  (params (OtherActor :type Actor%20Object%20Reference)))

(event EventTick
  (params (DeltaSeconds :type Float%20%28single-precision%29)))

(fn ConstructionScript)